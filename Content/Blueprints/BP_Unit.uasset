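; Selectable unit that the player can order to move to a location through its AI controller.
; Select and Deselect toggle a decal and add or remove the unit in the Selected array of BP_PlayerController.
; MoveTo forwards to MoveEvent in the event graph, where the latent AI MoveTo runs after stopping current movement.
; An invalid controller or failed move request prints a debug message.
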(event `MoveEvent`
  (params (Location :type "Vector Structure"))
  (bind _returnvalue (`AIBlueprintHelperLibrary.GetAIController` self))
  (if (`KismetSystemLibrary.IsValid` _returnvalue)
    (`Controller.StopMovement` _returnvalue)
    (`AITask_MoveTo.AIMoveTo` _returnvalue Location null
      (:`OnRequestFailed`
        (`KismetSystemLibrary.PrintText` "Move Failed" true true (struct :`R` 1.0 :`G` 0.167644 :`B` 0.287463 :`A` 1.0))))
    (else
      (`KismetSystemLibrary.PrintText` "AI Controller Invalid"))))

(fn `Deselect`
  (`SceneComponent.SetVisibility` (`self.Decal`) false false)
  (bind _asbp_player_controller (cast `/Game/Blueprints/BP_PlayerController` (`GameplayStatics.GetPlayerController` 0)))
  (`KismetArrayLibrary.Array_RemoveItem` (`/Game/Blueprints/BP_PlayerController.Selected` _asbp_player_controller) self))

(fn `MoveTo`
  (params (Location :type "Vector Structure"))
  (`self.MoveEvent` Location))

(fn `Select`
  (`SceneComponent.SetVisibility` (`self.Decal`) true false)
  (bind _asbp_player_controller (cast `/Game/Blueprints/BP_PlayerController` (`GameplayStatics.GetPlayerController` 0)))
  (`KismetArrayLibrary.Array_AddUnique` (`/Game/Blueprints/BP_PlayerController.Selected` _asbp_player_controller) self))

(fn `UserConstructionScript`
  (`parent.UserConstructionScript`))