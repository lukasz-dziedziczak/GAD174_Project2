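; BP_PlayerController is an RTS-style player controller for selecting units and ordering them to move.
; Left mouse clears the current selection and forwards press, per-tick hold and release messages to the HUD for marquee selection.
; Right click traces under the cursor, sends a move event to each selected BP_Unit and spawns a cursor effect there.
; Clearing calls Deselect on each selected BP_Selectable or BP_Unit before emptying the Selected array.
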(event `self.ReceiveBeginPlay`
  (`WidgetBlueprintLibrary.SetInputMode_GameAndUIEx` self null "LockAlways" false))

(event `self.ReceiveTick`
  (params (DeltaSeconds :type "Float (single-precision)"))
  (if (`self.IsLeftMousePressed?`)
    (message `/Game/Blueprints/BPI_RTSInterface.MarqueeHeld` (`self.GetHUD`))))

(event `Key|LeftMouseButton`
  (params (Key :type "Key Structure"))
  (bind _returnvalue (`self.GetHUD`))
  (:`Pressed`
    (set `self.IsLeftMousePressed?` true)
    (`self.ClearSelected`)
    (message `/Game/Blueprints/BPI_RTSInterface.MarqueePressed` _returnvalue))
  (:`Released`
    (set `self.IsLeftMousePressed?` false)
    (message `/Game/Blueprints/BPI_RTSInterface.MarqueeReleased` _returnvalue)))

(event `Key|RightMouseButton`
  (params (Key :type "Key Structure"))
  (bind _rightclicklocation (`self.RightClickLocation`))
  (:`Pressed`
    (set `self.RightClickLocation` (`.Location` (`GameplayStatics.BreakHitResult` (`self.GetHitResultUnderCursorByChannel` "TraceTypeQuery1"))))
    (for _array_element (`self.Selected`)
      (bind _asbp_unit (cast `/Game/Blueprints/BP_Unit` _array_element))
      (`/Game/Blueprints/BP_Unit.MoveEvent` _asbp_unit _rightclicklocation))
    (`NiagaraFunctionLibrary.SpawnSystemAtLocation` "/Game/Cursor/FX_Cursor.FX_Cursor" _rightclicklocation)))

(fn `ClearSelected`
  (bind _selected (`self.Selected`))
  (for _array_element _selected
    (bind _asbp_selectable (cast `/Game/Blueprints/BP_Selectable` _array_element)
      (:`then`
        (`/Game/Blueprints/BP_Selectable.Deselect` _asbp_selectable))
      (:`CastFailed`
        (bind _asbp_unit (cast `/Game/Blueprints/BP_Unit` _array_element))
        (`/Game/Blueprints/BP_Unit.Deselect` _asbp_unit))))
  (`KismetArrayLibrary.Array_Clear` _selected))

(fn `UserConstructionScript`)