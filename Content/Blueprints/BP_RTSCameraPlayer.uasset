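; RTS camera player that pans across the world by screen-edge scrolling and zooms with the mouse wheel.
; MouseX and MouseY events compare the cursor position to the viewport size and, within the outer 2% margins, offset the actor along world X or Y at ScrollSpeed scaled by delta time.
; Wheel presses step the SpringArm length by ZoomStep, clamped to a fixed range.
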(event `InputAxisKey|MouseX`
  (params (AxisValue :type "Float (single-precision)"))
  (bind _returnvalue_x (`KismetMathLibrary.BreakVector2D` (`WidgetLayoutLibrary.GetViewportSize`)))
  (bind _returnvalue (* (`self.ScrollSpeed`) (`GameplayStatics.GetWorldDeltaSeconds`)))
  (bind _returnvalue_2 (/ (`PlayerController.GetMousePosition` (`GameplayStatics.GetPlayerController` 0)) _returnvalue_x))
  (if (> _returnvalue_2 0.98)
    (`self.K2_AddActorWorldOffset` (`KismetMathLibrary.MakeVector` _returnvalue))
    (elif (< _returnvalue_2 0.02)
      (`self.K2_AddActorWorldOffset` (`KismetMathLibrary.MakeVector` (* _returnvalue -1.0))))))

(event `InputAxisKey|MouseY`
  (params (AxisValue :type "Float (single-precision)"))
  (bind (_returnvalue_x _returnvalue_y) (`KismetMathLibrary.BreakVector2D` (`WidgetLayoutLibrary.GetViewportSize`)))
  (bind _returnvalue (* (`self.ScrollSpeed`) (`GameplayStatics.GetWorldDeltaSeconds`)))
  (bind _returnvalue_2 (/ (`.LocationY` (`PlayerController.GetMousePosition` (`GameplayStatics.GetPlayerController` 0))) _returnvalue_y))
  (if (> _returnvalue_2 0.98)
    (`self.K2_AddActorWorldOffset` (`KismetMathLibrary.MakeVector` 0.0 _returnvalue))
    (elif (< _returnvalue_2 0.02)
      (`self.K2_AddActorWorldOffset` (`KismetMathLibrary.MakeVector` 0.0 (* _returnvalue -1.0))))))

(event `Key|MouseScrollUp`
  (params (Key :type "Key Structure"))
  (bind _springarm (`self.SpringArm`))
  (:`Pressed`
    (set `SpringArmComponent.TargetArmLength` (`KismetMathLibrary.FClamp` (- (`SpringArmComponent.TargetArmLength` _springarm) (`self.ZoomStep`)) 1000.0 6000.0) _springarm)))

(event `Key|MouseScrollDown`
  (params (Key :type "Key Structure"))
  (bind _springarm (`self.SpringArm`))
  (:`Pressed`
    (set `SpringArmComponent.TargetArmLength` (`KismetMathLibrary.FClamp` (+ (`SpringArmComponent.TargetArmLength` _springarm) (`self.ZoomStep`)) 1000.0 6000.0) _springarm)))

(fn `UserConstructionScript`)