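; BP_Selectable is a selectable Blueprint that shows or hides a decal to mark its selection state.
; Select shows the decal and adds itself uniquely to the Selected array on player 0's BP_PlayerController.
; Deselect hides the decal but also adds itself to that array instead of removing it.
; The event graph and construction script hold no logic.
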(fn `Deselect`
  (`SceneComponent.SetVisibility` (`self.Decal`) false false)
  (bind _asbp_player_controller (cast `/Game/Blueprints/BP_PlayerController` (`GameplayStatics.GetPlayerController` 0)))
  (`KismetArrayLibrary.Array_AddUnique` (`/Game/Blueprints/BP_PlayerController.Selected` _asbp_player_controller) self))

(fn `Select`
  (`SceneComponent.SetVisibility` (`self.Decal`) true false)
  (bind _asbp_player_controller (cast `/Game/Blueprints/BP_PlayerController` (`GameplayStatics.GetPlayerController` 0)))
  (`KismetArrayLibrary.Array_AddUnique` (`/Game/Blueprints/BP_PlayerController.Selected` _asbp_player_controller) self))

(fn `UserConstructionScript`)